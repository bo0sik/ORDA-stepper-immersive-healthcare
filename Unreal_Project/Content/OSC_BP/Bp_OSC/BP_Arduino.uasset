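; BP_Arduino is an actor that turns incoming OSC sensor and gaze messages into player character input.
; On BeginPlay it starts a listening OSC server and binds a handler that switches on each message's address path.
; Right and left sensor addresses trigger the matching step on BP_ThirdPersonCharacter, while gaze X sets GazeX and updates gaze yaw.
; An integer gaze-zone path and DoStep calls are left disconnected, and OSCServerRef is unused.
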(event `self.ReceiveBeginPlay`
  (bind _returnvalue (`OSCManager.CreateOSCServer` "0.0.0.0" 10000 false true "" self))
  (add `OSCServer.OnOscMessageReceived` _returnvalue (delegate `Message Received`)))

(event `Message Received`
  (params (Message :type "OSCMessage Structure (by ref)") (IPAddress :type String) (Port :type Integer))
  (bind _returnvalue (`GameplayStatics.GetPlayerCharacter` 0))
  (bind _returnvalue_2 (`OSCManager.GetOSCMessageAddress` Message))
  (bind _returnvalue_3 (`OSCManager.GetOSCAddressFullPath` _returnvalue_2))
  (switch `string` _returnvalue_3
    (:`/sensor/right_up`
      (bind _asbp_third_person_character (cast `/Game/ThirdPerson/Blueprints/BP_ThirdPersonCharacter` _returnvalue))
      (`/Game/ThirdPerson/Blueprints/BP_ThirdPersonCharacter.RightStepFromSensor` _asbp_third_person_character))
    (:`/sensor/left_up`
      (bind _asbp_third_person_character_2 (cast `/Game/ThirdPerson/Blueprints/BP_ThirdPersonCharacter` _returnvalue))
      (`/Game/ThirdPerson/Blueprints/BP_ThirdPersonCharacter.LeftStepFromSensor` _asbp_third_person_character_2))
    (:`/gaze/x`
      (bind _value (`OSCManager.GetFloat` Message))
      (bind _asbp_third_person_character_3 (cast `/Game/ThirdPerson/Blueprints/BP_ThirdPersonCharacter` (`GameplayStatics.GetPlayerCharacter` 0)))
      (bind _output_get (set `/Game/ThirdPerson/Blueprints/BP_ThirdPersonCharacter.GazeX` _value _asbp_third_person_character_3))
      (`/Game/ThirdPerson/Blueprints/BP_ThirdPersonCharacter.SetGazeYawFromX` _asbp_third_person_character_3 _output_get))))

(fn `UserConstructionScript`)